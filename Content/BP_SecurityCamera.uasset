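; Security camera actor that sweeps side to side and spawns a guard enemy when its trigger box is overlapped.
; A self-restarting timeline ping-pongs the camera mesh yaw between two limits.
; Each tick, a debug-drawn trace along the scene capture's view places the StatusLED decal on the surface hit.
; Any box overlap sets the decal material, stops the sweep, and spawns BP_GuardEnemy once at that impact point.
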(event `self.ReceiveBeginPlay`
  (bind (_relativerotation_roll _relativerotation_pitch) (`KismetMathLibrary.BreakRotator` (`SceneComponent.RelativeRotation` (`self.SM_Camera`))))
  (bind (_direction _moving_value) (`Timeline|Timeline` :!label _label)
    (:`Update`
      (`SceneComponent.K2_SetRelativeRotation` (`self.SM_Camera`) (`KismetMathLibrary.RLerp` (`KismetMathLibrary.MakeRotator` _relativerotation_roll _relativerotation_pitch -45.0) (`KismetMathLibrary.MakeRotator` _relativerotation_roll _relativerotation_pitch 45.0) _moving_value) false false))
    (:`Finished`
      (if (`self.Restart?`)
        (set `self.Restart?` false)
        (goto _label)
        (else
          (set `self.Restart?` true)
          (goto _label :!via `Reverse`))))))

(event `Block Timeline`
  (goto _label :!via `Stop`))

(event `self.ReceiveTick`
  (params (DeltaSeconds :type "Float (single-precision)"))
  (bind _returnvalue (`SceneComponent.K2_GetComponentLocation` (`self.SceneCaptureComponent2D`)))
  (bind _outhit (`KismetSystemLibrary.LineTraceSingle` :`Start` _returnvalue :`End` (+ (* (`SceneComponent.GetForwardVector` (`self.SceneCaptureComponent2D`)) 1000.0) _returnvalue) :`TraceChannel` "TraceTypeQuery1" :`DrawDebugType` "ForOneFrame"))
  (bind (_bblockinghit _binitialoverlap _time _distance _location _impactpoint _normal _impactnormal) (`GameplayStatics.BreakHitResult` _outhit))
  (`SceneComponent.K2_SetWorldLocationAndRotation` (`self.StatusLED`) _impactpoint (`KismetMathLibrary.Conv_VectorToRotator` _impactnormal) false false))

(event `self.Box.OnComponentBeginOverlap`
  (params (OverlappedComponent :type "PrimitiveComponent Object Reference") (OtherActor :type "Actor Object Reference") (OtherComp :type "PrimitiveComponent Object Reference") (OtherBodyIndex :type Integer) (bFromSweep :type Boolean) (SweepResult :type "HitResult Structure (by ref)"))
  (`DecalComponent.SetDecalMaterial` (`self.StatusLED`) null)
  (`self.Block Timeline`)
  (if (not (`self.Spawned?`))
    (`|SpawnActorFromClass` "/Game/Blueprints/GuardCharacter/BP_GuardEnemy.BP_GuardEnemy_C" (`KismetMathLibrary.MakeTransform` (`.ImpactPoint` (`GameplayStatics.BreakHitResult` (stale `self.ReceiveTick` _outhit)))) "Undefined" "MultiplyWithRoot" null null))
  (set `self.Spawned?` true))

(fn `UserConstructionScript`)