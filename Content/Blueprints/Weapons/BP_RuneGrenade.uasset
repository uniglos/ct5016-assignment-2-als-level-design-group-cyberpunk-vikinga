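; Thrown rune grenade that detonates on a short timed fuse.
; A one-shot Throw event detaches it, launches it through ProjectileMovement with the given velocity, and moves the Sphere component toward a random rotation.
; Sphere1 collision starts disabled from construction and turns on shortly after release.
; When the fuse ends, ExplosiveComponent explodes, Sphere is hidden, and the actor gets a short lifespan before cleanup.
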(event `Throw`
  (params (Velocity :type "Vector Structure"))
  (bind _projectilemovement (`self.ProjectileMovement`))
  (`/Engine/EditorBlueprintResources/StandardMacros.DoOnce` false
    (:`Completed`
      (`|ExecutionSequence`
        (:`then_0`
          (`self.K2_DetachFromActor` "KeepWorld" "KeepWorld" "KeepWorld")
          (set `MovementComponent.Velocity` Velocity _projectilemovement)
          (`ActorComponent.Activate` _projectilemovement false)
          (`KismetSystemLibrary.Delay` 0.2)
          (`PrimitiveComponent.SetCollisionEnabled` (`self.Sphere1`) "QueryAndPhysics")
          (`KismetSystemLibrary.Delay` 1.0)
          (`/Game/Blueprints/Weapons/ExplosiveComponent.Explode` (`self.ExplosiveComponent`))
          (`SceneComponent.SetHiddenInGame` (`self.Sphere`) true false)
          (`self.SetLifeSpan` 3.0))
        (:`then_1`
          (`KismetSystemLibrary.MoveComponentTo` (`self.Sphere`) (0.0 0.0 0.0) (`KismetMathLibrary.RandomRotator` false)))))))

(fn `UserConstructionScript`
  (`PrimitiveComponent.SetCollisionEnabled` (`self.Sphere1`) "NoCollision"))