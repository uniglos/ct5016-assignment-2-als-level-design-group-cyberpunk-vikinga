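; An actor component for weapons that makes its owning actor explode once, damaging nearby pawns and destructibles.
; Explode is guarded by DoOnce and spawns grenade-launcher particles, sound and a randomly rotated, downward-facing decal at the owner's location.
; A zero-length multi-sphere trace of ExplodeRadius collects unique actors, each receiving fixed ExplosiveDamage that is also reported as an AI damage-sense event.
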(event `Explode`
  (bind _returnvalue (`self.GetOwner`))
  (bind _returnvalue_2 (`self.GetOwner`))
  (bind _returnvalue_3 (`Actor.K2_GetActorLocation` _returnvalue))
  (bind _returnvalue_4 (`SceneComponent.K2_GetComponentLocation` (`Actor.RootComponent` _returnvalue)))
  (`/Engine/EditorBlueprintResources/StandardMacros.DoOnce` false
    (:`Completed`
      (`GameplayStatics.SpawnEmitterAtLocation` "/Game/PrototypeWeap/FX/P_GrenadeLauncher_Explosion_01.P_GrenadeLauncher_Explosion_01" _returnvalue_3)
      (`GameplayStatics.PlaySoundAtLocation` "/Game/PrototypeWeap/Sound/GrenadeLauncher/GL_Explosion01.GL_Explosion01" _returnvalue_3 (struct) 1.0 1.0 0.0 null null null null)
      (`GameplayStatics.SpawnDecalAtLocation` "/Game/Materials/MAT_BulletDecal.MAT_BulletDecal" (0.0 0.0 0.0) _returnvalue_3 (`KismetMathLibrary.MakeRotator` 0.0 -90.0 (`KismetMathLibrary.RandomFloatInRange` 0.0 360.0)))
      (bind (_outhits _returnvalue_5) (`KismetSystemLibrary.SphereTraceMultiForObjects` _returnvalue_4 _returnvalue_4 (`self.ExplodeRadius`) (`|MakeArray` "ObjectTypeQuery3" "ObjectTypeQuery6" :!type "EObjectTypeQuery Enum")))
      (if _returnvalue_5
        (for _array_element _outhits
          (`KismetArrayLibrary.Array_AddUnique` (`self.NearbyActors`) (`.HitActor` (`GameplayStatics.BreakHitResult` _array_element))))
        (for _array_element_2 (`self.NearbyActors`)
          (bind _returnvalue_6 (`GameplayStatics.ApplyDamage` _array_element_2 200.0 null _returnvalue_2 "/Game/Mechanics/ExplosiveDamage.ExplosiveDamage_C"))
          (`AISense_Damage.ReportDamageEvent` _array_element_2 _returnvalue_2 _returnvalue_6 (`Actor.K2_GetActorLocation` _returnvalue_2)))))))